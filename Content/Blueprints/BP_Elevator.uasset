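; BP_Elevator is an elevator actor that travels one way to a Target actor's location once the player enters its trigger.
; Overlap of TriggerElevate by BP_PlayerCharacter sets IsElevating, and Tick then moves the actor toward Target at constant MoveSpeed with sweep.
; When the next step would reach or overshoot, it snaps to Target and stops.
; The construction script stores InitialPosition, which no graph here reads.
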(event `self.ReceiveTick`
  (params (DeltaSeconds :type "Float (single-precision)"))
  (bind _returnvalue_location (`KismetMathLibrary.BreakTransform` (`self.GetTransform`)))
  (bind _returnvalue_location_2 (`KismetMathLibrary.BreakTransform` (`self.GetTransform` (`self.Target`))))
  (bind _returnvalue_location_3 (`KismetMathLibrary.BreakTransform` (`self.GetTransform` (`self.Target`))))
  (bind _returnvalue (* DeltaSeconds (`self.MoveSpeed`)))
  (bind _returnvalue_2 (- _returnvalue_location_3 _returnvalue_location))
  (if (`self.IsElevating`)
    ;[1 1 1] Check if target is reached
    (if (>= _returnvalue (`KismetMathLibrary.VSize` _returnvalue_2))
      ;[1 1 1] Finish elevating
      (`self.K2_SetActorLocation` _returnvalue_location_2)
      (set `self.IsElevating` false)
      (else
        ;[1 1 1] Move towards target
        (`self.K2_AddActorWorldTransform` (`KismetMathLibrary.MakeTransform` (* (`KismetMathLibrary.Normal` _returnvalue_2) _returnvalue)) true)))))

(event `self.TriggerElevate.OnComponentBeginOverlap`
  (params (OverlappedComponent :type "PrimitiveComponent Object Reference") (OtherActor :type "Actor Object Reference") (OtherComp :type "PrimitiveComponent Object Reference") (OtherBodyIndex :type Integer) (bFromSweep :type Boolean) (SweepResult :type "HitResult Structure (by ref)"))
  ;[1 1 1] Trigger movement
  (cast `/Game/Blueprints/Character/BP_PlayerCharacter` OtherActor)
  (set `self.IsElevating` true))

(fn `UserConstructionScript`
  (set `self.InitialPosition` (`self.GetTransform`)))